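; BP_Bullet is a projectile actor that deals damage to the first other actor it overlaps, then destroys itself.
; Overlaps with its instigator are ignored, a check flagged to change to class or team.
; The construction script feeds the gravity scale and speed variables into the ProjectileMovement component and sets the bullet's lifespan.
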(event Collision|EventActorBeginOverlap
  (params (OtherActor :type Actor%20Object%20Reference))
  (if (== OtherActor (Game|GetInstigator))
    (Development|PrintString "INSTIGATOR SELF COLLISION" false false "(R=1.000000,G=0.000000,B=0.044042,A=1.000000)")
    (else
      (Game|Damage|ApplyDamage OtherActor (Variables|Default|GetDamage) (Game|GetInstigatorController) self)
      (Actor|DestroyActor))))

(fn ConstructionScript
  (bind _projectilemovement (Variables|Default|GetProjectileMovement))
  (Variables|/Script/Engine.ProjectileMovementComponent|SetProjectileGravityScale _projectilemovement (Variables|Default|GetGravityScale))
  (Variables|/Script/Engine.ProjectileMovementComponent|SetInitialSpeed _projectilemovement (Variables|Default|GetProjectileSpeed))
  (Actor|SetLifeSpan (Variables|Default|GetLifetime)))