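; 2D platform built from Paper2D sprite tiles, with a Soft type that the player can pass through from its trigger side.
; The construction script tiles left, middle and right sprites between two rounded widget positions and sizes DownTrigger to that span.
; When BP_ProPlayer overlaps DownTrigger, Soft parts ignore GameTraceChannel2, then block it again on exit.
; A BlockProjectiles flag sets whether parts block GameTraceChannel1.
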(event OnComponentBeginOverlap(DownTrigger)
  (params (OtherActor :type Actor%20Object%20Reference) (OtherComp :type Primitive%20Component%20Object%20Reference) (OtherBodyIndex :type Integer) (bFromSweep :type Boolean) (SweepResult :type Hit%20Result%20Structure%20%28by%20ref%29))
  (Utilities|Casting|CastToBP_ProPlayer OtherActor
    (:then
      (switch Utilities|FlowControl|Switch|SwitchonPlatformType (Variables|Default|GetPlatformType)
        (:NewEnumerator1
          (for _array_element (Variables|Default|GetPlatform%20Parts%20Array)
            (Collision|SetCollisionResponsetoChannel _array_element "ECC_GameTraceChannel2" "ECR_Ignore")))))
    (:CastFailed
      (Development|PrintString (Utilities|String|Append "WARNING " (Utilities|GetObjectName OtherActor)) true true "(R=1.000000,G=0.098612,B=0.390662,A=1.000000)"))))

(event OnComponentEndOverlap(DownTrigger)
  (params (OtherActor :type Actor%20Object%20Reference) (OtherComp :type Primitive%20Component%20Object%20Reference) (OtherBodyIndex :type Integer))
  (Utilities|Casting|CastToBP_ProPlayer OtherActor)
  (switch Utilities|FlowControl|Switch|SwitchonPlatformType (Variables|Default|GetPlatformType)
    (:NewEnumerator1
      (for _array_element (Variables|Default|GetPlatform%20Parts%20Array)
        (Collision|SetCollisionResponsetoChannel _array_element "ECC_GameTraceChannel2" "ECR_Block")))))

(event EventBeginPlay
  (for _array_element (Variables|Default|GetPlatform%20Parts%20Array)
    (Collision|SetCollisionEnabled _array_element "QueryAndPhysics")))

(fn ConstructionScript
  (bind _triggeroffset (Variables|Default|GetTriggerOffset))
  (bind _triggerscale (Variables|Default|GetTriggerScale))
  (Variables|Default|SetRoundedLeftWidget (CallFunction|RoundVector (Variables|Default|GetPlatform%20Left%20Widget)))
  (Variables|Default|SetRoundedRightWidget (CallFunction|RoundVector (Variables|Default|GetPlatform%20Right%20Widget)))
  (Utilities|FlowControl|Sequence
    (:then_0
      (Components|Box|SetBoxExtent (Variables|Default|GetDownTrigger) (Math|Vector|MakeVector (/ (- (.x (Variables|Default|GetRoundedRightWidget)) (.x (Variables|Default|GetRoundedLeftWidget))) 2.0) (.y _triggerscale) (.z _triggerscale)) true)
      (Transformation|SetRelativeLocation (Variables|Default|GetDownTrigger) (Math|Vector|MakeVector (/ (+ (.x (Variables|Default|GetRoundedRightWidget)) (.x (Variables|Default|GetRoundedLeftWidget))) 2.0) (.y _triggeroffset) (Utilities|CalculateTriggerZOffset (.z _triggeroffset) (Variables|Default|GetAutoOffsetTriggerZ))) false false))
    (:then_1
      (for _index (range 0 (- (Math|Float|Floor (/ (- (.x (Variables|Default|GetRoundedRightWidget)) (.x (Variables|Default|GetRoundedLeftWidget))) (Variables|Default|GetSpacing))) 1))
        (bind _index_2 (Utilities|CompareIndexMacro _index 0 (- (Math|Float|Floor (/ (- (.x (Variables|Default|GetRoundedRightWidget)) (.x (Variables|Default|GetRoundedLeftWidget))) (Variables|Default|GetSpacing))) 1))
          (:Left
            (CallFunction|AddNewPart _index_2 (Variables|Default|GetLeftSprite)))
          (:Right
            (CallFunction|AddNewPart _index_2 (Variables|Default|GetRightSprite)))
          (:Mid
            (CallFunction|AddNewPart _index_2 (Variables|Default|GetMidSprite))))))))

(fn AddNewPart
  (params (Index :type Integer) (Sprite :type Paper%20Sprite%20Object%20Reference))
  (bind _spacing (Variables|Default|GetSpacing))
  (bind _returnvalue (AddComponent|AddPaperSpriteComponent false (Math|Transform|MakeTransform (Math|Vector|MakeVector (+ (+ (* Index _spacing) (/ _spacing 2.0)) (.x (Variables|Default|GetRoundedLeftWidget))) 0.0 0.0) "0.000000, 0, 0" "1,1,1")))
  (Utilities|Array|Add (Variables|Default|GetPlatform%20Parts%20Array) _returnvalue)
  (Rendering|Components|Sprite|SetSprite _returnvalue Sprite)
  (Collision|SetCollisionEnabled _returnvalue "QueryAndPhysics")
  (Collision|SetCollisionObjectType _returnvalue "ECC_GameTraceChannel4")
  (Collision|SetCollisionResponsetoChannel _returnvalue "ECC_GameTraceChannel4" "ECR_Ignore")
  (Collision|SetCollisionResponsetoChannel _returnvalue "ECC_GameTraceChannel1" (select (Variables|Default|GetBlockProjectiles) "ECR_Block" "ECR_Ignore")))

(fn RoundVector
  (params (Vector :type Vector))
  (return (Math|Vector|MakeVector (Math|Conversions|ToFloat(Integer) (Math|Float|Round (.x Vector))) (Math|Conversions|ToFloat(Integer) (Math|Float|Round (.y Vector))) (Math|Conversions|ToFloat(Integer) (Math|Float|Round (.z Vector))))))

(fn SetBlockProjectiles
  (params (BlockProjectiles :type Boolean))
  (Variables|Default|SetBlockProjectiles BlockProjectiles)
  (for _array_element (Variables|Default|GetPlatform%20Parts%20Array)
    (Collision|SetCollisionResponsetoChannel _array_element "ECC_GameTraceChannel1" (select BlockProjectiles "ECR_Block" "ECR_Ignore"))))