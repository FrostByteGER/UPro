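; Game mode for an endless platformer that procedurally spawns BP_Platform actors ahead of the player.
; BeginPlay derives jump limits from character movement and places a starting platform at the player start.
; Tick adds platforms within one screen width, using projectile-motion math for reachable gaps and heights, randomly adds monsters, and destroys passed off-screen platforms.
; CheatMode adds invincibility and a following safety platform; world-origin shifting exists but is disconnected.
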(event Custom|CustomEvent_0
  (params (SelfActor :type Actor%20Object%20Reference) (OtherActor :type Actor%20Object%20Reference) (NormalImpulse :type Vector) (Hit :type Hit%20Result%20Structure%20%28by%20ref%29))
  (bind _returnvalue (Viewport|GetViewportSize))
  (bind _returnvalue_2 (Game|GetPlayerController 0))
  (bind (_worldposition _worlddirection _returnvalue_3) (Class|GameplayStatics|DeprojectScreentoWorld _returnvalue_2 (Math|Vector2D|MakeVector2D (.x _returnvalue) 0.0)))
  (Utilities|Casting|CastToBP_ProPlayer OtherActor)
  (Collision|UnbindEventfromOnActorHit (stale EventBeginPlay _platform) (delegate Custom|CustomEvent_0))
  ;[1 1 1] Remember screen width in world coords
  (if _returnvalue_3
    (Variables|Default|SetViewportWorldSizeX (Math|Float|Absolute(Float) (- (.x _worldposition) (.x (Transformation|GetActorLocation (Game|GetPlayerController 0))))))))

(event EventBeginPlay
  (bind _returnvalue (Game|GetPlayerCharacter 0))
  (bind _playerstartlocation (Variables|Default|GetPlayerStartLocation))
  (bind _charactermovement (Variables|/Script/Engine.Character|GetCharacterMovement _returnvalue))
  (bind _returnvalue_2 (Components|Movement|GetGravityZ _charactermovement))
  (bind _jumpzvelocity (Variables|/Script/Engine.CharacterMovementComponent|GetJumpZVelocity _charactermovement))
  ;[1 1 1] Calculate Jump Distance and Height
  (Variables|Default|SetGravityPositive (Math|Float|Absolute(Float) _returnvalue_2))
  (Variables|Default|SetMaxJumpDistance (* (* (|((2*v)/g) _jumpzvelocity _returnvalue_2) -1.0) (Variables|/Script/Engine.CharacterMovementComponent|GetMaxWalkSpeed _charactermovement)))
  (Variables|Default|SetMaxJumpHeight (* (|((v*v)/(2*g)) _jumpzvelocity _returnvalue_2) -1.0))
  (bind _asbp_pro_player (Utilities|Casting|CastToBP_ProPlayer (Game|GetPlayerCharacter 0)))
  (Variables|/Game/Pro/Blueprints/BP_ProPlayer.BP_ProPlayer_C|SetInvincible _asbp_pro_player (Variables|Default|GetCheatMode))
  ;[1 1 1] Spawn initial Platform
  (bind _platform (CallFunction|CreatePlatform (+ (.x _playerstartlocation) -1e+02) (+ (.z _playerstartlocation) -5e+01) 2e+02 "NewEnumerator0"))
  (Collision|BindEventtoOnActorHit _platform (delegate Custom|CustomEvent_0))
  (if (Variables|Default|GetCheatMode)
    ;[1 1 1] Spawn Invincibility Platform to keep player alive
    (bind _returnvalue_3 (Game|SpawnActorfromClass "/Game/Pro/Blueprints/BP_Platform.BP_Platform_C" (Math|Transform|MakeTransform (Math|Vector|MakeVector 0.0 0.0 (+ (Variables|Default|GetPlatformMinHeight) -5e+01)) "0, 0, 0" "1,1,1") "Undefined" 0 "NewEnumerator0" "0.000000,0.000000,0.000000" (Math|Vector|MakeVector 2e+02 0.0 0.0) true true false 0))))

(event EventTick
  (params (DeltaSeconds :type Float%20%28single-precision%29))
  (Utilities|FlowControl|Sequence
    (:then_0
      ;[1 1 1] Spawn Invincibility Platform to keep player alive
      (if (Variables|Default|GetCheatMode)
        (Transformation|SetActorLocation (stale EventBeginPlay _returnvalue_3) (Math|Vector|MakeVector (- (.x (Transformation|GetActorLocation (Game|GetPlayerCharacter 0))) 1e+02) (.y (Transformation|GetActorLocation (stale EventBeginPlay _returnvalue_3))) (.z (Transformation|GetActorLocation (stale EventBeginPlay _returnvalue_3)))) false false)))
    (:then_1
      ;[1 1 1] Create next platform if in range
      (if (< (Math|Float|Absolute(Float) (- (.x (Transformation|GetActorLocation (Game|Player|GetPlayerPawn 0))) (Variables|Default|GetCurrentPlatformSpawnPositionX))) (Variables|Default|GetViewportWorldSizeX))
        (bind (_spawntransform_location_x _spawntransform_location_z _platform_width _platformtype) (CallFunction|CalculatePlatformSpawnData))
        (CallFunction|CreatePlatform _spawntransform_location_x _spawntransform_location_z _platform_width _platformtype)
        ;[1 1 1] Mob Spawning on Platform
        (if (> (Math|Random|RandomFloat) (Variables|Default|GetPlatformMobSpawnChance))
          _
          (else
            (CallFunction|SpawnMonster)))
        (Development|PrintString "New Platform Spawned!")
        (CallFunction|RemovePassedPlatforms)))))

(fn ConstructionScript)

(fn ShiftWorldOrigin
  (bind _returnvalue (Game|GetPlayerCharacter 0))
  (bind _worldoriginshiftthreshold (Variables|Default|GetWorldOriginShiftThreshold))
  (bind _returnvalue_2 (Transformation|GetActorLocation _returnvalue))
  (if (or (> (.x _returnvalue_2) _worldoriginshiftthreshold) (< (.x _returnvalue_2) (* _worldoriginshiftthreshold -1.0)))
    (Class|GameplayStatics|SetWorldOriginLocation (Utilities|Struct|MakeIntVector (+ (Math|Float|Truncate (.x _returnvalue_2)) (.x (Class|GameplayStatics|GetWorldOriginLocation))) 0 0))))

(fn CalculatePlatformSpawnData
  (bind _returnvalue (Game|GetPlayerCharacter 0))
  (bind _currentplatformspawnpositionz (Variables|Default|GetCurrentPlatformSpawnPositionZ))
  (bind _platformmingap (Variables|Default|GetPlatformMinGap))
  (bind _maxjumpdistance (Variables|Default|GetMaxJumpDistance))
  (bind _currentplatformspawnpositionx (Variables|Default|GetCurrentPlatformSpawnPositionX))
  (bind _platformxthreshold (Variables|Default|GetPlatformXThreshold))
  (bind _platformzthreshold (Variables|Default|GetPlatformZThreshold))
  (bind _returnvalue_2 (Math|Random|RandomFloatinRange _platformmingap _maxjumpdistance))
  (bind _charactermovement (Variables|/Script/Engine.Character|GetCharacterMovement _returnvalue))
  ;[0 1 0] Width
  (Variables|Default|SetPreviousPlatformWidth (Variables|Default|GetCurrentPlatformWidth))
  ;[1 0 0] Position
  (bind _output_get (Variables|Default|SetCurrentPlatformGap (select (> _returnvalue_2 _platformxthreshold) (- _returnvalue_2 _platformxthreshold) _returnvalue_2)))
  (Variables|Default|SetPreviousPlatformSpawnPositionX _currentplatformspawnpositionx)
  ;[0 0 1] Height
  (Variables|Default|SetPreviousPlatformSpawnPositionZ _currentplatformspawnpositionz)
  (return (+ _currentplatformspawnpositionx (Variables|Default|GetPreviousPlatformWidth) _output_get) (select (> (Math|Random|RandomFloatinRange (Variables|Default|GetPlatformMinHeight) (|(h+((Vy*t)-((0.500000*g)*(t*t)))) (Variables|/Script/Engine.CharacterMovementComponent|GetJumpZVelocity _charactermovement) (Variables|Default|GetGravityPositive) (|(x/Vx) (Variables|Default|GetCurrentPlatformGap) (Variables|/Script/Engine.CharacterMovementComponent|GetMaxWalkSpeed _charactermovement)) _currentplatformspawnpositionz)) _platformzthreshold) (- (Math|Random|RandomFloatinRange (Variables|Default|GetPlatformMinHeight) (|(h+((Vy*t)-((0.500000*g)*(t*t)))) (Variables|/Script/Engine.CharacterMovementComponent|GetJumpZVelocity _charactermovement) (Variables|Default|GetGravityPositive) (|(x/Vx) (Variables|Default|GetCurrentPlatformGap) (Variables|/Script/Engine.CharacterMovementComponent|GetMaxWalkSpeed _charactermovement)) _currentplatformspawnpositionz)) _platformzthreshold) (Math|Random|RandomFloatinRange (Variables|Default|GetPlatformMinHeight) (|(h+((Vy*t)-((0.500000*g)*(t*t)))) (Variables|/Script/Engine.CharacterMovementComponent|GetJumpZVelocity _charactermovement) (Variables|Default|GetGravityPositive) (|(x/Vx) (Variables|Default|GetCurrentPlatformGap) (Variables|/Script/Engine.CharacterMovementComponent|GetMaxWalkSpeed _charactermovement)) _currentplatformspawnpositionz))) (Math|Random|RandomFloatinRange (Variables|Default|GetPlatformMinWidth) (Variables|Default|GetPlatformMaxWidth)) (select (> (Variables|Default|GetCurrentPlatformSpawnPositionZ) (+ (Variables|Default|GetPreviousPlatformSpawnPositionZ) (Variables|Default|GetSoftPlatformMinHeightThreshold))) "NewEnumerator1" "NewEnumerator0")))

(fn SpawnMonster
  (Game|SpawnActorfromClass "/Game/Pro/Blueprints/BP_Monster.BP_Monster_C" (Math|Transform|MakeTransform (Math|Vector|MakeVector (+ (Variables|Default|GetCurrentPlatformSpawnPositionX) (/ (Variables|Default|GetCurrentPlatformWidth) 2.0)) 0.0 (+ (Variables|Default|GetCurrentPlatformSpawnPositionZ) 2e+01)) "0, 0, 0" "1,1,1") "Undefined" 0 (select (> (Math|Random|RandomFloat) 0.5) "1.000000,0,0" "-1.000000,0,0") 0))

(fn RemovePassedPlatforms
  (bind _array_element (Utilities|Array|ForEachLoopwithBreak (Variables|Default|GetPlatforms) :!label _label)
    (:LoopBody
      (if (< (.X (Math|Vector|BreakVector (Default|GetEndPartWorldPosition _array_element))) (.x (Transformation|GetActorLocation (Game|Player|GetPlayerPawn 0))))
        (if (< (.x (.ScreenPosition (Class|GameplayStatics|ProjectWorldtoScreen (Game|GetPlayerController 0) (Default|GetEndPartWorldPosition _array_element) false))) (LocalVariables|GetPositionOffsetX))
          (Utilities|Array|Add (LocalVariables|GetPlatformsToRemove) _array_element))
        (else
          (goto _label Break))))
    (:Completed
      (for _array_element_2 (LocalVariables|GetPlatformsToRemove)
        (Utilities|Array|RemoveItem (Variables|Default|GetPlatforms) _array_element_2)
        (Actor|DestroyActor _array_element_2)))))

(fn CreatePlatform
  (params (SpawnTransform_Location_X :type Float%20%28single-precision%29) (SpawnTransform_Location_Z :type Float%20%28single-precision%29) (Platform%20Width :type Float%20%28single-precision%29) (PlatformType :type PlatformType%20Enum :default "NewEnumerator0"))
  (Variables|Default|SetCurrentPlatformSpawnPositionX SpawnTransform_Location_X)
  (Variables|Default|SetCurrentPlatformSpawnPositionZ SpawnTransform_Location_Z)
  (Variables|Default|SetCurrentPlatformWidth Platform%20Width)
  (bind _returnvalue (Game|SpawnActorfromClass "/Game/Pro/Blueprints/BP_Platform.BP_Platform_C" (Math|Transform|MakeTransform (Math|Vector|MakeVector SpawnTransform_Location_X 0.0 SpawnTransform_Location_Z) "0, 0, 0" "1,1,1") "Undefined" 0 PlatformType "0.000000,0.000000,0.000000" (Math|Vector|MakeVector Platform%20Width 0.0 0.0) true true false 0))
  (Utilities|Array|Add (Variables|Default|GetPlatforms) _returnvalue)
  (return _returnvalue))

(fn ChoosePlayerStart
  (params (Player :type Controller%20Object%20Reference))
  (bind _returnvalue (|CallParentFunction Player))
  (Variables|Default|SetPlayerStartLocation (Transformation|GetActorLocation _returnvalue))
  (return _returnvalue))